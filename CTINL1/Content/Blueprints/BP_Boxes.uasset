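; BP_Boxes is a breakable box that takes two hits from BP_Ball or BP_ExtraBall and awards a point.
; On BeginPlay it moves its Cube to a fixed height, keeping X and Y.
; The first ball overlap sets HitBefore and toggles the visibility of Cube and GCIcePlatform.
; A later overlap waits briefly, increments Points on BP_MainPlayer and destroys the box.
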(event OnComponentBeginOverlap(Box)
  (params (OverlappedComponent :type Primitive%20Component%20Object%20Reference) (OtherActor :type Actor%20Object%20Reference) (OtherComp :type Primitive%20Component%20Object%20Reference) (OtherBodyIndex :type Integer) (bFromSweep :type Boolean) (SweepResult :type Hit%20Result%20Structure%20%28by%20ref%29))
  (Utilities|Casting|CastToBP_Ball OtherActor
    (:then
      _)
    (:CastFailed
      (Utilities|Casting|CastToBP_ExtraBall OtherActor)))
  (if (Variables|Default|GetHitBefore)
    (Utilities|FlowControl|Delay 0.5)
    (bind _asbp_main_player (Utilities|Casting|CastToBP_MainPlayer (Game|Player|GetPlayerPawn 0)))
    (Variables|/Game/Blueprints/BP_MainPlayer.BP_MainPlayer_C|SetPoints _asbp_main_player (+ (Variables|/Game/Blueprints/BP_MainPlayer.BP_MainPlayer_C|GetPoints _asbp_main_player) 1))
    (Actor|DestroyActor)
    (else
      (Variables|Default|SetHitBefore true)
      (Rendering|ToggleVisibility (Variables|Default|GetCube) false)
      (Rendering|ToggleVisibility (Variables|Default|GetGC_IcePlatform) false))))

(event EventBeginPlay
  (bind _cube (Variables|Default|GetCube))
  (bind _returnvalue (Transformation|GetWorldLocation _cube))
  ;[0.15 0.15 0.15 0.5] Get position
  (Variables|Default|SetPointsBox 0)
  (Transformation|SetWorldLocation _cube (Math|Vector|MakeVector (.x _returnvalue) (.y _returnvalue) 1e+02) false false))

(fn ConstructionScript)