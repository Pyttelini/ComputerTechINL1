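; BP_MainPlayer is the touch-controlled player bar that slides horizontally in a game with BP_Ball.
; While a finger is down, Tick traces under it and copies the hit's X to the bar, keeping Y and using a fixed height.
; An Enhanced Input double tap triggers an action on the ball, gated by a delay-based cooldown.
; BeginPlay adds a dynamic snow post-process material to the camera, with a timeline driving its density.
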(event Custom|Snow%20Post%20Process
  (bind _newtrack_0 (Timeline|Timeline PlayFromStart)
    (:Update
      (Rendering|Material|SetScalarParameterValue (Variables|Components|GetDynamic%20Post%20Process) "Density" _newtrack_0 :!class /Script/Engine.MaterialInstanceDynamic))))

(event Input|EnhancedActionEvents|EnhancedInputActionIA_doubletapp
  (params (ActionValue :type Boolean) (ElapsedSeconds :type Float%20%28double-precision%29) (TriggeredSeconds :type Float%20%28double-precision%29) (InputAction :type Input%20Action%20Object%20Reference :default "/Game/FilippasBlueprints/IA_doubletapp.IA_doubletapp"))
  (:Completed
    (if (Variables|Default|GetDoubleTapped)
      (bind _returnvalue (Actor|GetActorOfClass "/Game/Blueprints/BP_Ball.BP_Ball_C"))
      (Default|Doubbletapp _returnvalue)
      (Variables|Default|SetDoubleTapped false)
      (Utilities|FlowControl|Delay 1e+01)
      (Variables|Default|SetDoubleTapped true)
      (else
        (Utilities|FlowControl|Delay 5.0)
        (Variables|Default|SetDoubleTapped true)))))

(event EventControllerChanged
  (params (OldController :type Controller%20Object%20Reference) (NewController :type Controller%20Object%20Reference))
  (bind _asplayer_controller (Utilities|Casting|CastToPlayerController NewController))
  (Input|AddMappingContext (PlayerController|LocalPlayerSubsystems|GetEnhancedInputLocalPlayerSubsystem _asplayer_controller) "/Game/FilippasBlueprints/IA_inputsystem.IA_inputsystem" 0 "(bIgnoreAllPressedKeysUntilRelease=True,bForceImmediately=False,bNotifyUserSettings=False)"))

(event EventTick
  (params (DeltaSeconds :type Float%20%28single-precision%29))
  (bind _player (Variables|Default|GetPlayer))
  (bind _player_2 (Variables|Default|GetPlayer))
  ;[0.15 0.15 0.15 0.5] Swipe to move bar
  (if (Variables|Default|GetIsTouching)
    (Transformation|SetWorldLocation _player_2 (Math|Vector|MakeVector (.X (Math|Vector|BreakVector (.location (.HitResult (Class|PlayerController|GetHitResultUnderFingerbyChannel (Game|GetPlayerController 0) "Touch1" "TraceTypeQuery1" true))))) (.y (Transformation|GetWorldLocation _player_2)) 1e+02) false false)
    (else
      ;[0.15 0.15 0.15 0.5] If finger leaves screen
      (Transformation|SetWorldLocation _player (Transformation|GetWorldLocation _player) false false))))

(event EventBeginPlay
  (bind _returnvalue (Rendering|Material|CreateDynamicMaterialInstance "/Game/GRA/Ai/M_Snow.M_Snow" "None" "None" :!class /Script/Engine.KismetMaterialLibrary))
  (bind _output_get (Variables|Components|SetDynamic%20Post%20Process _returnvalue))
  (Utilities|Struct|SetmembersinPostProcessSettings (Variables|/Script/Engine.CameraComponent|GetPostProcessSettings (Variables|Default|GetCamera)) (Utilities|Struct|MakeWeightedBlendables (Utilities|Array|MakeArray (Utilities|Struct|MakeWeightedBlendable 1.0 _output_get))))
  (CallFunction|SnowPostProcess))

(event Input|TouchEvents|InputTouch
  (params (Location :type Vector) (FingerIndex :type ETouchIndex%20Enum))
  ;[0.15 0.15 0.15 0.5] Check if finger is touching
  (:Pressed
    (Variables|Default|SetIsTouching true))
  (:Released
    (Variables|Default|SetIsTouching false)))

(fn ConstructionScript)