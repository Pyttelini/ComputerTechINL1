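; BP_Ball is a ball actor that launches itself at game start and can temporarily spawn extra balls.
; On BeginPlay it sets the Sphere's height, keeping its X and Y, then applies a one-off impulse along positive Y.
; The Doubletapp event spawns two BP_ExtraBall actors at the Sphere's location and destroys both after a five-second delay.
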(event Custom|Doubbletapp
  (bind _sphere (Variables|Default|GetSphere))
  (bind _returnvalue (Transformation|GetWorldLocation _sphere))
  (bind _returnvalue_2 (Game|SpawnActorfromClass "/Game/FilippasBlueprints/BP_ExtraBall.BP_ExtraBall_C" (Math|Transform|MakeTransform _returnvalue "0, 0, 0" "1.000000,1.000000,1.000000") "Undefined" "MultiplyWithRoot" 0 0))
  (bind _returnvalue_3 (Game|SpawnActorfromClass "/Game/FilippasBlueprints/BP_ExtraBall.BP_ExtraBall_C" (Math|Transform|MakeTransform _returnvalue "0, 0, 0" "1.000000,1.000000,1.000000") "Undefined" "MultiplyWithRoot" 0 0))
  (Utilities|FlowControl|Delay 5.0)
  (Actor|DestroyActor _returnvalue_2))

(event EventBeginPlay
  (bind _sphere (Variables|Default|GetSphere))
  (bind _returnvalue (Transformation|GetWorldLocation _sphere))
  (Transformation|SetWorldLocation _sphere (Math|Vector|MakeVector (.x _returnvalue) (.y _returnvalue) 1e+02) false false)
  (Physics|AddImpulse _sphere "0.000000,1000.000000,0.000000" "None" false))

(event Collision|EventActorBeginOverlap
  (params (OtherActor :type Actor%20Object%20Reference)))

(event EventTick
  (params (DeltaSeconds :type Float%20%28single-precision%29)))

(fn ConstructionScript)