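; BP_AILVL adds a snow post-process effect to the player camera when play begins; despite its name, it holds no AI logic.
; BeginPlay creates a dynamic instance of M_Snow and sets it as a full-weight post-process blendable on PlayerCamera.
; SnowPostProcess then plays a Timeline that drives the material's Density parameter over time.
; Debug strings print at startup and on every Timeline update.
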(event Custom|Snow%20Post%20Process
  (bind _newtrack_0 (Timeline|Timeline PlayFromStart)
    (:Update
      (Development|PrintString (Utilities|String|ToString(Float) _newtrack_0))
      (Rendering|Material|SetScalarParameterValue (Variables|Default|GetDynamic%20Post%20Process) "Density" _newtrack_0 :!class /Script/Engine.MaterialInstanceDynamic))))

(event EventBeginPlay
  (Development|PrintString "Begin!!! AI version" true true "(R=0.000000,G=0.660000,B=1.000000,A=1.000000)" 2e+01)
  (bind _returnvalue (Rendering|Material|CreateDynamicMaterialInstance "/Game/GRA/Ai/M_Snow.M_Snow" "None" "None" :!class /Script/Engine.KismetMaterialLibrary))
  (bind _output_get (Variables|Default|SetDynamic%20Post%20Process _returnvalue))
  (Utilities|Struct|SetmembersinPostProcessSettings (Variables|/Script/Engine.CameraComponent|GetPostProcessSettings (Variables|Default|GetPlayerCamera)) (Utilities|Struct|MakeWeightedBlendables (Utilities|Array|MakeArray (Utilities|Struct|MakeWeightedBlendable 1.0 _output_get))))
  (Development|PrintString "KÖR" true true "(R=0.000000,G=0.660000,B=1.000000,A=1.000000)" 2e+01)
  (CallFunction|SnowPostProcess))

(fn ConstructionScript)